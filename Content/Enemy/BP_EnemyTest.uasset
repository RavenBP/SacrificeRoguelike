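; BP_EnemyTest is a test enemy that takes projectile hits and melee-attacks the player while in range.
; Projectile overlaps on the capsule destroy the projectile and subtract the player's attack from health stored on the healthbar widget, destroying the enemy at zero.
; A radius sphere toggles healthbar visibility.
; The melee radius sets CanAttack, starting a delay-driven loop that damages the player every cooldown until they leave.
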(event OnComponentBeginOverlap(Capsule)
  (params (OverlappedComponent :type Primitive%20Component%20Object%20Reference) (OtherActor :type Actor%20Object%20Reference) (OtherComp :type Primitive%20Component%20Object%20Reference) (OtherBodyIndex :type Integer) (bFromSweep :type Boolean) (SweepResult :type Hit%20Result%20Structure%20%28by%20ref%29))
  ;[1 1 1] Hit by Projectile
  (bind _asfirst_person_projectile (Utilities|Casting|CastToFirstPersonProjectile OtherActor))
  (Actor|DestroyActor _asfirst_person_projectile)
  (CallFunction|TakeDamage))

(event OnComponentBeginOverlap(HealthBarRadius)
  (params (OverlappedComponent :type Primitive%20Component%20Object%20Reference) (OtherActor :type Actor%20Object%20Reference) (OtherComp :type Primitive%20Component%20Object%20Reference) (OtherBodyIndex :type Integer) (bFromSweep :type Boolean) (SweepResult :type Hit%20Result%20Structure%20%28by%20ref%29))
  ;[1 1 1] Healthbar Visibility
  (Utilities|Casting|CastToFirstPersonCharacter OtherActor)
  (Rendering|SetVisibility (Variables|Default|GetWidget) true false))

(event OnComponentEndOverlap(HealthBarRadius)
  (params (OverlappedComponent :type Primitive%20Component%20Object%20Reference) (OtherActor :type Actor%20Object%20Reference) (OtherComp :type Primitive%20Component%20Object%20Reference) (OtherBodyIndex :type Integer))
  ;[1 1 1] Healthbar Visibility
  (Utilities|Casting|CastToFirstPersonCharacter OtherActor)
  (Rendering|SetVisibility (Variables|Default|GetWidget) false false))

(event OnComponentBeginOverlap(MeleeAttackRadius)
  (params (OverlappedComponent :type Primitive%20Component%20Object%20Reference) (OtherActor :type Actor%20Object%20Reference) (OtherComp :type Primitive%20Component%20Object%20Reference) (OtherBodyIndex :type Integer) (bFromSweep :type Boolean) (SweepResult :type Hit%20Result%20Structure%20%28by%20ref%29))
  (Utilities|Casting|CastToFirstPersonCharacter OtherActor)
  (Variables|Default|SetcanAttack true)
  (CallFunction|AttackPlayer))

(event OnComponentEndOverlap(MeleeAttackRadius)
  (params (OverlappedComponent :type Primitive%20Component%20Object%20Reference) (OtherActor :type Actor%20Object%20Reference) (OtherComp :type Primitive%20Component%20Object%20Reference) (OtherBodyIndex :type Integer))
  (Utilities|Casting|CastToFirstPersonCharacter OtherActor)
  (Variables|Default|SetcanAttack false))

(event Custom|TakeDamage
  (bind _healthbarref (Variables|Default|GetHealthbarREF))
  ;[1 1 1] Take Damage
  (bind _asfirst_person_character (Utilities|Casting|CastToFirstPersonCharacter (Game|Player|GetPlayerPawn 0)))
  (bind _output_get (Variables|/Game/UI/EnemyHealthbarUI.EnemyHealthbarUI_C|SetenemyCurrentHealth _healthbarref (- (Variables|/Game/UI/EnemyHealthbarUI.EnemyHealthbarUI_C|GetenemyCurrentHealth _healthbarref) (Variables|/Game/FirstPersonBP/Blueprints/FirstPersonCharacter.FirstPersonCharacter_C|GetplayerAttack _asfirst_person_character))))
  (if (<= _output_get 0.0)
    (Actor|DestroyActor)))

(event Custom|AttackPlayer
  ;[1 1 1] Enemy Attack
  (Utilities|FlowControl|Delay 0.5) ; Time of Animation could go here
  (if (Variables|Default|GetcanAttack) :!label _label
    (bind _asfirst_person_character (Utilities|Casting|CastToFirstPersonCharacter (Game|Player|GetPlayerPawn 0)))
    (Default|TookDamage _asfirst_person_character (Variables|Default|Getattack))
    (Utilities|FlowControl|Delay (Variables|Default|GetattackCooldown))
    (goto _label)
    (else
      (Development|PrintString "Player dodged attack"))))

(event EventBeginPlay
  (bind _enemystats (Variables|Default|GetEnemyStats))
  (bind (_enemytype _health _attack _speed) (Utilities|Struct|BreakEnemyStruct _enemystats))
  ;[1 1 1] Initialization
  (bind _output_get (Variables|Default|SetmaxHealth 1e+02))
  (Variables|Default|SetcurrentHealth 75.0)
  (Variables|Default|Setattack _attack)
  (Variables|Default|Setspeed _speed)
  (bind _asenemy_healthbar_ui (Utilities|Casting|CastToEnemyHealthbarUI (UserInterface|GetUserWidgetObject (Variables|Default|GetWidget))))
  (Variables|Default|SetHealthbarREF _asenemy_healthbar_ui)
  (bind _output_get_2 (Variables|/Game/UI/EnemyHealthbarUI.EnemyHealthbarUI_C|SetenemyMaxHealth _asenemy_healthbar_ui _output_get))
  (Variables|/Game/UI/EnemyHealthbarUI.EnemyHealthbarUI_C|SetenemyCurrentHealth _asenemy_healthbar_ui _output_get_2))

(fn ConstructionScript
  (Components|Sphere|SetSphereRadius (Variables|Default|GetHealthBarRadius) (Variables|Default|GethealthBarRange) true))