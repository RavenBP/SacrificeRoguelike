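; Melee enemy that chases the player on sight via pawn sensing and AIMoveTo, with health, attack and speed initialized from EnemyStats.
; Projectile hits and overlaps with the player's melee collision subtract PlayerAttack from health kept in the healthbar widget, destroying the enemy at zero.
; Construction-sized spheres toggle healthbar visibility and start a delayed attack loop that repeats on cooldown while the player stays in range.
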(event OnSeePawn(PawnSensing)
  (params (Pawn :type Pawn%20Object%20Reference))
  (bind _asfirst_person_character (Utilities|Casting|CastToFirstPersonCharacter Pawn))
  (AI|AIMoveTo self "0, 0, 0" _asfirst_person_character 5.0 false))

(event OnComponentBeginOverlap(HealthBarRadius)
  (params (OverlappedComponent :type Primitive%20Component%20Object%20Reference) (OtherActor :type Actor%20Object%20Reference) (OtherComp :type Primitive%20Component%20Object%20Reference) (OtherBodyIndex :type Integer) (bFromSweep :type Boolean) (SweepResult :type Hit%20Result%20Structure%20%28by%20ref%29))
  ;[1 1 1] Healthbar Visibility
  (Utilities|Casting|CastToFirstPersonCharacter OtherActor)
  (Rendering|SetVisibility (Variables|Default|GetWidget) true false))

(event OnComponentEndOverlap(HealthBarRadius)
  (params (OverlappedComponent :type Primitive%20Component%20Object%20Reference) (OtherActor :type Actor%20Object%20Reference) (OtherComp :type Primitive%20Component%20Object%20Reference) (OtherBodyIndex :type Integer))
  ;[1 1 1] Healthbar Visibility
  (Utilities|Casting|CastToFirstPersonCharacter OtherActor)
  (Rendering|SetVisibility (Variables|Default|GetWidget) false false))

(event OnComponentBeginOverlap(CapsuleComponent)
  (params (OverlappedComponent :type Primitive%20Component%20Object%20Reference) (OtherActor :type Actor%20Object%20Reference) (OtherComp :type Primitive%20Component%20Object%20Reference) (OtherBodyIndex :type Integer) (bFromSweep :type Boolean) (SweepResult :type Hit%20Result%20Structure%20%28by%20ref%29))
  ;[1 1 1] This only works if collision is (Pawn->WorldDynamic)... need to research why
  (if (and (== OtherComp (Variables|Default|GetMelee%20Collision)) (not (Variables|Default|GettookMeleeDamage)))
    (Variables|Default|SettookMeleeDamage true)
    (CallFunction|TakeDamage)
    (Utilities|FlowControl|Delay 0.6)
    (Variables|Default|SettookMeleeDamage false)))

(event OnComponentBeginOverlap(AttackRadius)
  (params (OverlappedComponent :type Primitive%20Component%20Object%20Reference) (OtherActor :type Actor%20Object%20Reference) (OtherComp :type Primitive%20Component%20Object%20Reference) (OtherBodyIndex :type Integer) (bFromSweep :type Boolean) (SweepResult :type Hit%20Result%20Structure%20%28by%20ref%29))
  (Utilities|Casting|CastToFirstPersonCharacter OtherActor)
  (Variables|Default|SetcanAttack true)
  (CallFunction|AttackPlayer))

(event OnComponentEndOverlap(AttackRadius)
  (params (OverlappedComponent :type Primitive%20Component%20Object%20Reference) (OtherActor :type Actor%20Object%20Reference) (OtherComp :type Primitive%20Component%20Object%20Reference) (OtherBodyIndex :type Integer))
  (Utilities|Casting|CastToFirstPersonCharacter OtherActor)
  (Variables|Default|SetcanAttack false))

(event OnComponentHit(CapsuleComponent)
  (params (HitComponent :type Primitive%20Component%20Object%20Reference) (OtherActor :type Actor%20Object%20Reference) (OtherComp :type Primitive%20Component%20Object%20Reference) (NormalImpulse :type Vector :default "0, 0, 0") (Hit :type Hit%20Result%20Structure%20%28by%20ref%29))
  (bind _asfirst_person_projectile (Utilities|Casting|CastToFirstPersonProjectile OtherActor))
  (Actor|DestroyActor _asfirst_person_projectile)
  (CallFunction|TakeDamage))

(event Custom|TakeDamage
  (bind _healthbarref (Variables|Default|GetHealthbarREF))
  ;[1 1 1] Take Damage
  (bind _asfirst_person_character (Utilities|Casting|CastToFirstPersonCharacter (Game|Player|GetPlayerPawn 0)))
  (bind _output_get (Variables|/Game/UI/EnemyHealthbarUI.EnemyHealthbarUI_C|SetenemyCurrentHealth _healthbarref (- (Variables|/Game/UI/EnemyHealthbarUI.EnemyHealthbarUI_C|GetenemyCurrentHealth _healthbarref) (Variables|/Game/FirstPersonBP/Blueprints/FirstPersonCharacter.FirstPersonCharacter_C|GetplayerAttack _asfirst_person_character))))
  (if (<= _output_get 0.0)
    (Actor|DestroyActor)))

(event Custom|AttackPlayer
  ;[1 1 1] Attack Player
  (if (not (Variables|Default|GetisAttacking))
    (Variables|Default|SetisAttacking true)
    (Utilities|FlowControl|Delay 0.5) ; Time of Animation could go here
    (if (Variables|Default|GetcanAttack) :!label _label
      (bind _asfirst_person_character (Utilities|Casting|CastToFirstPersonCharacter (Game|Player|GetPlayerPawn 0)))
      (Default|TookDamage _asfirst_person_character (Variables|Default|Getattack))
      (Utilities|FlowControl|Delay (Variables|Default|GetattackCooldown))
      (goto _label)
      (else
        (Development|PrintString "Player dodged attack")
        (Variables|Default|SetisAttacking false)))))

(event EventBeginPlay
  (bind _enemystats (Variables|Default|GetenemyStats))
  (bind (_enemytype _health _attack _speed) (Utilities|Struct|BreakEnemyStruct _enemystats))
  ;[1 1 1] Initialization
  (bind _asfirst_person_character (Utilities|Casting|CastToFirstPersonCharacter (Game|Player|GetPlayerPawn 0)))
  (Variables|Default|SetMelee%20Collision (Variables|/Game/FirstPersonBP/Blueprints/FirstPersonCharacter.FirstPersonCharacter_C|GetMeleeCollision _asfirst_person_character))
  (bind _output_get (Variables|Default|SetmaxHealth _health))
  (Variables|Default|SetcurrentHealth _output_get)
  (Variables|Default|Setattack _attack)
  (Variables|/Script/Engine.CharacterMovementComponent|SetMaxWalkSpeed (Variables|Character|GetCharacterMovement) _speed)
  (bind _asenemy_healthbar_ui (Utilities|Casting|CastToEnemyHealthbarUI (UserInterface|GetUserWidgetObject (Variables|Default|GetWidget))))
  (bind _output_get_2 (Variables|Default|SetHealthbarREF _asenemy_healthbar_ui))
  (bind _output_get_3 (Variables|/Game/UI/EnemyHealthbarUI.EnemyHealthbarUI_C|SetenemyMaxHealth _output_get_2 _output_get))
  (Variables|/Game/UI/EnemyHealthbarUI.EnemyHealthbarUI_C|SetenemyCurrentHealth _asenemy_healthbar_ui _output_get_3))

(fn ConstructionScript
  (Components|Sphere|SetSphereRadius (Variables|Default|GetAttackRadius) (Variables|Default|GetmeleeAttackRange) true)
  (Components|Sphere|SetSphereRadius (Variables|Default|GetHealthBarRadius) (Variables|Default|GethealthBarRange) true))