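; BP_Turret is an enemy turret that turns to face the player when seen and fires projectiles on a one-second cooldown.
; BeginPlay loads health, attack and speed from EnemyStats and initializes a healthbar widget, which shows while the player is inside HealthBarRadius.
; Player projectile hits and cooldown-gated melee overlaps call TakeDamage, which subtracts PlayerAttack from the widget's health value and destroys the turret at zero.
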(event OnSeePawn(PawnSensing)
  (params (Pawn :type Pawn%20Object%20Reference))
  (bind _asfirst_person_character (Utilities|Casting|CastToFirstPersonCharacter Pawn))
  (Utilities|FlowControl|Sequence
    (:then_0
      (Transformation|SetActorRotation (Math|Rotator|FindLookatRotation (Transformation|GetActorLocation) (Transformation|GetActorLocation _asfirst_person_character))))
    (:then_1
      (if (Variables|Default|GetspawnProjectile)
        (bind _returnvalue (Game|SpawnActorfromClass "/Game/FirstPersonBP/Blueprints/EnemyProjectile.EnemyProjectile_C" (Transformation|GetWorldTransform (Variables|Default|GetProjectileSpawnLocation)) "Undefined" 0 0))
        (Variables|/Game/FirstPersonBP/Blueprints/EnemyProjectile.EnemyProjectile_C|Setdamage _returnvalue (Variables|Default|Getattack))
        (Physics|AddImpulse (Variables|/Game/FirstPersonBP/Blueprints/EnemyProjectile.EnemyProjectile_C|GetSphere _returnvalue) (* (Math|Vector|GetForwardVector (Variables|Default|GetStaticMesh)) (Variables|Default|GetprojectileForce)) "None" true)
        (Variables|Default|SetspawnProjectile false)
        (Utilities|FlowControl|Delay 1.0)
        (Variables|Default|SetspawnProjectile true)))))

(event OnComponentBeginOverlap(HealthBarRadius)
  (params (OverlappedComponent :type Primitive%20Component%20Object%20Reference) (OtherActor :type Actor%20Object%20Reference) (OtherComp :type Primitive%20Component%20Object%20Reference) (OtherBodyIndex :type Integer) (bFromSweep :type Boolean) (SweepResult :type Hit%20Result%20Structure%20%28by%20ref%29))
  ;[1 1 1] Healthbar Visibility
  (Utilities|Casting|CastToFirstPersonCharacter OtherActor)
  (Rendering|SetVisibility (Variables|Default|GetWidget) true false))

(event OnComponentEndOverlap(HealthBarRadius)
  (params (OverlappedComponent :type Primitive%20Component%20Object%20Reference) (OtherActor :type Actor%20Object%20Reference) (OtherComp :type Primitive%20Component%20Object%20Reference) (OtherBodyIndex :type Integer))
  ;[1 1 1] Healthbar Visibility
  (Utilities|Casting|CastToFirstPersonCharacter OtherActor)
  (Rendering|SetVisibility (Variables|Default|GetWidget) false false))

(event OnComponentBeginOverlap(CapsuleComponent)
  (params (OverlappedComponent :type Primitive%20Component%20Object%20Reference) (OtherActor :type Actor%20Object%20Reference) (OtherComp :type Primitive%20Component%20Object%20Reference) (OtherBodyIndex :type Integer) (bFromSweep :type Boolean) (SweepResult :type Hit%20Result%20Structure%20%28by%20ref%29))
  ;[1 1 1] This only works if collision is (Pawn->WorldDynamic)... need to research why
  (if (and (== OtherComp (Variables|Default|GetMelee%20Collision)) (not (Variables|Default|GettookMeleeDamage)))
    (Variables|Default|SettookMeleeDamage true)
    (CallFunction|TakeDamage)
    (Utilities|FlowControl|Delay 0.6)
    (Variables|Default|SettookMeleeDamage false)))

(event OnComponentHit(CapsuleComponent)
  (params (HitComponent :type Primitive%20Component%20Object%20Reference) (OtherActor :type Actor%20Object%20Reference) (OtherComp :type Primitive%20Component%20Object%20Reference) (NormalImpulse :type Vector :default "0, 0, 0") (Hit :type Hit%20Result%20Structure%20%28by%20ref%29))
  (bind _asfirst_person_projectile (Utilities|Casting|CastToFirstPersonProjectile OtherActor))
  (Actor|DestroyActor _asfirst_person_projectile)
  (CallFunction|TakeDamage))

(event Custom|TakeDamage
  (bind _healthbarref (Variables|Default|GetHealthbarREF))
  ;[1 1 1] Take Damage
  (bind _asfirst_person_character (Utilities|Casting|CastToFirstPersonCharacter (Game|Player|GetPlayerPawn 0)))
  (bind _output_get (Variables|/Game/UI/EnemyHealthbarUI.EnemyHealthbarUI_C|SetenemyCurrentHealth _healthbarref (- (Variables|/Game/UI/EnemyHealthbarUI.EnemyHealthbarUI_C|GetenemyCurrentHealth _healthbarref) (Variables|/Game/FirstPersonBP/Blueprints/FirstPersonCharacter.FirstPersonCharacter_C|GetplayerAttack _asfirst_person_character))))
  (if (<= _output_get 0.0)
    (Actor|DestroyActor)))

(event EventBeginPlay
  (bind _enemystats (Variables|Default|GetenemyStats))
  (bind (_enemytype _health _attack _speed) (Utilities|Struct|BreakEnemyStruct _enemystats))
  ;[1 1 1] Initialization
  (bind _asfirst_person_character (Utilities|Casting|CastToFirstPersonCharacter (Game|Player|GetPlayerPawn 0)))
  (Variables|Default|SetMelee%20Collision (Variables|/Game/FirstPersonBP/Blueprints/FirstPersonCharacter.FirstPersonCharacter_C|GetMeleeCollision _asfirst_person_character))
  (bind _output_get (Variables|Default|SetmaxHealth _health))
  (Variables|Default|SetcurrentHealth _output_get)
  (Variables|Default|Setattack _attack)
  (Variables|/Script/Engine.CharacterMovementComponent|SetMaxWalkSpeed (Variables|Character|GetCharacterMovement) _speed)
  (bind _asenemy_healthbar_ui (Utilities|Casting|CastToEnemyHealthbarUI (UserInterface|GetUserWidgetObject (Variables|Default|GetWidget))))
  (bind _output_get_2 (Variables|Default|SetHealthbarREF _asenemy_healthbar_ui))
  (bind _output_get_3 (Variables|/Game/UI/EnemyHealthbarUI.EnemyHealthbarUI_C|SetenemyMaxHealth _output_get_2 _output_get))
  (Variables|/Game/UI/EnemyHealthbarUI.EnemyHealthbarUI_C|SetenemyCurrentHealth _asenemy_healthbar_ui _output_get_3))

(fn ConstructionScript
  (Components|Sphere|SetSphereRadius (Variables|Default|GetAttackRadius) 0.0 true)
  (Components|Sphere|SetSphereRadius (Variables|Default|GetHealthBarRadius) (Variables|Default|GethealthBarRange) true))