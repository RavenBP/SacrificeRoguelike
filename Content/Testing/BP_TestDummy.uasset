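; Test dummy actor that tallies damage from the first-person player and displays the running total.
; On BeginPlay it caches the player character's MeleeCollision.
; Its TakeDmg event adds the player's PlayerAttack to DmgTaken and updates a "DMG TAKEN" text.
; Both overlap events are empty; melee-detection debug prints and projectile destroy-and-damage logic are disconnected, so TakeDmg has no live caller within this Blueprint.
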(event OnComponentBeginOverlap(Box)
  (params (OverlappedComponent :type Primitive%20Component%20Object%20Reference) (OtherActor :type Actor%20Object%20Reference) (OtherComp :type Primitive%20Component%20Object%20Reference) (OtherBodyIndex :type Integer) (bFromSweep :type Boolean) (SweepResult :type Hit%20Result%20Structure%20%28by%20ref%29)))

(event Custom|TakeDmg
  (bind _asfirst_person_character (Utilities|Casting|CastToFirstPersonCharacter (Game|Player|GetPlayerPawn 0)))
  ;[1 1 1] Should the projectile or the player do dmg? Should both be taken into effect??
  (bind _output_get (Variables|Default|SetdmgTaken (+ (Variables|Default|GetdmgTaken) (Variables|/Game/FirstPersonBP/Blueprints/FirstPersonCharacter.FirstPersonCharacter_C|GetplayerAttack _asfirst_person_character))))
  (Rendering|Components|TextRender|SetText (Variables|Default|GetDmgTakenText) (Utilities|Text|ToText(String) (Utilities|String|Append "DMG TAKEN: " (Utilities|String|ToString(Float) _output_get)))))

(event EventBeginPlay
  (bind _asfirst_person_character (Utilities|Casting|CastToFirstPersonCharacter (Game|Player|GetPlayerPawn 0)))
  (Variables|Default|SetMelee%20Collision (Variables|/Game/FirstPersonBP/Blueprints/FirstPersonCharacter.FirstPersonCharacter_C|GetMeleeCollision _asfirst_person_character)))

(event Collision|EventActorBeginOverlap
  (params (OtherActor :type Actor%20Object%20Reference)))

(fn ConstructionScript)