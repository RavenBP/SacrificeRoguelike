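; BP_StrikeSelect is a testing pickup-style selector that sets how many strikes the player has remaining.
; On BeginPlay its TextRender displays the NumStrikes value.
; When the FirstPersonCharacter overlaps its Sphere, it writes NumStrikes into StrikesRemaining on SacrificeGameInstance and prints a debug confirmation.
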(event OnComponentBeginOverlap(Sphere)
  (params (OverlappedComponent :type Primitive%20Component%20Object%20Reference) (OtherActor :type Actor%20Object%20Reference) (OtherComp :type Primitive%20Component%20Object%20Reference) (OtherBodyIndex :type Integer) (bFromSweep :type Boolean) (SweepResult :type Hit%20Result%20Structure%20%28by%20ref%29))
  (Utilities|Casting|CastToFirstPersonCharacter OtherActor)
  (bind _assacrifice_game_instance (Utilities|Casting|CastToSacrificeGameInstance (Game|GetGameInstance)))
  (Variables|/Game/Gameplay/SacrificeGameInstance.SacrificeGameInstance_C|SetstrikesRemaining _assacrifice_game_instance (Variables|Default|GetnumStrikes))
  (Development|PrintString "Num Strikes Set"))

(event EventBeginPlay
  (Rendering|Components|TextRender|SetText (Variables|Default|GetTextRender) (Utilities|Text|ToText(Integer) (Variables|Default|GetnumStrikes))))

(fn ConstructionScript)