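; BP_Cluster is a cluster actor whose static mesh appears on activation and whose sphere detects a nearby first-person character.
; The construction script sizes the sphere from ClusterActivationRadius, toggles the text label, and sets mesh visibility and collision from IsActivated.
; Activate reveals the mesh with query-only collision unless IsActivated is true, but never sets that flag.
; Player overlap only prints a message; a TookDamage call is left unconnected.
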(event OnComponentBeginOverlap(Sphere)
  (params (OverlappedComponent :type Primitive%20Component%20Object%20Reference) (OtherActor :type Actor%20Object%20Reference) (OtherComp :type Primitive%20Component%20Object%20Reference) (OtherBodyIndex :type Integer) (bFromSweep :type Boolean) (SweepResult :type Hit%20Result%20Structure%20%28by%20ref%29))
  (bind _asfirst_person_character (Utilities|Casting|CastToFirstPersonCharacter OtherActor))
  (Development|PrintString "Player within cluster range"))

(event Custom|Activate
  (bind _staticmesh (Variables|Default|GetStaticMesh))
  (if (Variables|Default|GetisActivated)
    (Development|PrintString "Cluster already activated")
    (else
      (Rendering|SetVisibility _staticmesh true false)
      (Collision|SetCollisionEnabled _staticmesh "QueryOnly"))))

(fn ConstructionScript
  (bind _staticmesh (Variables|Default|GetStaticMesh))
  (Components|Sphere|SetSphereRadius (Variables|Default|GetSphere) (Variables|Default|GetclusterActivationRadius) true)
  (Rendering|SetVisibility (Variables|Default|GetTextRender) (Variables|Default|GetdisplayText) false)
  (if (Variables|Default|GetisActivated)
    (Rendering|SetVisibility _staticmesh true false)
    (Collision|SetCollisionEnabled _staticmesh "QueryOnly")
    (else
      (Rendering|SetVisibility _staticmesh false false)
      (Collision|SetCollisionEnabled _staticmesh "NoCollision"))))