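; BP_Stairs is a level-exit interactable that makes the player choose a debuff card before moving on to the next level.
; Its Box overlap shows or hides the interact prompt and toggles actor input for the first-person character.
; Pressing E stores LevelToLoad in SacrificeGameInstance and opens a DebuffCardSelection widget filled with three entries from its Card array.
; It then hides the gameplay UI, switches to UI-only mouse input and disables the Box collision.
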(event OnComponentBeginOverlap(Box)
  (params (OverlappedComponent :type Primitive%20Component%20Object%20Reference) (OtherActor :type Actor%20Object%20Reference) (OtherComp :type Primitive%20Component%20Object%20Reference) (OtherBodyIndex :type Integer) (bFromSweep :type Boolean) (SweepResult :type Hit%20Result%20Structure%20%28by%20ref%29))
  (bind _asfirst_person_character (Utilities|Casting|CastToFirstPersonCharacter OtherActor))
  (Default|DisplayInteractUI (Variables|/Game/FirstPersonBP/Blueprints/FirstPersonCharacter.FirstPersonCharacter_C|GetGameplayUI _asfirst_person_character))
  (Input|EnableInput (Game|GetPlayerController 0)))

(event OnComponentEndOverlap(Box)
  (params (OverlappedComponent :type Primitive%20Component%20Object%20Reference) (OtherActor :type Actor%20Object%20Reference) (OtherComp :type Primitive%20Component%20Object%20Reference) (OtherBodyIndex :type Integer))
  (bind _asfirst_person_character (Utilities|Casting|CastToFirstPersonCharacter OtherActor))
  (Default|RemoveInteractUI (Variables|/Game/FirstPersonBP/Blueprints/FirstPersonCharacter.FirstPersonCharacter_C|GetGameplayUI _asfirst_person_character))
  (Input|DisableInput (Game|GetPlayerController 0)))

(event Input|KeyboardEvents|E
  (params (Key :type Key%20Structure))
  (bind _returnvalue (Game|GetPlayerController 0))
  (bind _card (Variables|Default|GetCard))
  (:Pressed
    (bind _assacrifice_game_instance (Utilities|Casting|CastToSacrificeGameInstance (Game|GetGameInstance)))
    (Variables|/Game/Gameplay/SacrificeGameInstance.SacrificeGameInstance_C|SetnextLevelName _assacrifice_game_instance (Variables|Default|GetLevelToLoad))
    (bind _returnvalue_2 (UserInterface|CreateWidget "/Game/UI/DebuffCards/DebuffCardSelection.DebuffCardSelection_C"))
    (Variables|/Game/UI/DebuffCards/DebuffCardUI.DebuffCardUI_C|SetCardInfo (Variables|/Game/UI/DebuffCards/DebuffCardSelection.DebuffCardSelection_C|GetDebuffCardUI _returnvalue_2) (Utilities|Array|Get(acopy) _card))
    (Variables|/Game/UI/DebuffCards/DebuffCardUI.DebuffCardUI_C|SetCardInfo (Variables|/Game/UI/DebuffCards/DebuffCardSelection.DebuffCardSelection_C|GetDebuffCardUI_1 _returnvalue_2) (Utilities|Array|Get(acopy) _card 1))
    (Variables|/Game/UI/DebuffCards/DebuffCardUI.DebuffCardUI_C|SetCardInfo (Variables|/Game/UI/DebuffCards/DebuffCardSelection.DebuffCardSelection_C|GetDebuffCardUI_2 _returnvalue_2) (Utilities|Array|Get(acopy) _card 2))
    (UserInterface|Viewport|AddtoViewport _returnvalue_2 0)
    (bind _asfirst_person_character (Utilities|Casting|CastToFirstPersonCharacter (Game|Player|GetPlayerPawn 0)))
    (Widget|SetVisibility (Variables|/Game/FirstPersonBP/Blueprints/FirstPersonCharacter.FirstPersonCharacter_C|GetGameplayUI _asfirst_person_character) "Hidden")
    (bind _output_get (Variables|/Game/FirstPersonBP/Blueprints/FirstPersonCharacter.FirstPersonCharacter_C|SetCardSelectionUI _asfirst_person_character _returnvalue_2))
    (Input|SetInputModeUIOnly _returnvalue _output_get "DoNotLock")
    (Variables|/Script/Engine.PlayerController|SetbShowMouseCursor _returnvalue true)
    (Collision|SetCollisionEnabled (Variables|Default|GetBox) "NoCollision")))

(fn ConstructionScript)