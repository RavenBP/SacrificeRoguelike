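; BP_Pickup is an item pickup that grants the first-person character bonus health, attack and speed.
; The construction script builds floating stat labels from the bonus values, leaving any zero stat blank.
; Overlapping its sphere shows the prompt and stat texts and enables input on the actor, while leaving reverses both.
; Pressing E passes the bonuses to the character's UpdateStats and destroys the pickup.
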(event OnComponentBeginOverlap(Sphere)
  (params (OverlappedComponent :type Primitive%20Component%20Object%20Reference) (OtherActor :type Actor%20Object%20Reference) (OtherComp :type Primitive%20Component%20Object%20Reference) (OtherBodyIndex :type Integer) (bFromSweep :type Boolean) (SweepResult :type Hit%20Result%20Structure%20%28by%20ref%29))
  (Utilities|Casting|CastToFirstPersonCharacter OtherActor)
  (Rendering|SetVisibility (Variables|Default|GetTextRender) true false)
  (Input|EnableInput (Game|GetPlayerController 0)))

(event OnComponentEndOverlap(Sphere)
  (params (OverlappedComponent :type Primitive%20Component%20Object%20Reference) (OtherActor :type Actor%20Object%20Reference) (OtherComp :type Primitive%20Component%20Object%20Reference) (OtherBodyIndex :type Integer))
  (Utilities|Casting|CastToFirstPersonCharacter OtherActor)
  (Rendering|SetVisibility (Variables|Default|GetTextRender) false false)
  (Input|DisableInput (Game|GetPlayerController 0)))

(event EventBeginPlay
  (Rendering|SetVisibility (Variables|Default|GetTextRender) false false))

(event Input|KeyboardEvents|E
  (params (Key :type Key%20Structure :default "None"))
  (:Pressed
    (Development|PrintString "Player picked up item")
    (bind _asfirst_person_character (Utilities|Casting|CastToFirstPersonCharacter (Game|Player|GetPlayerPawn 0)))
    (Default|UpdateStats _asfirst_person_character (Variables|Default|GetAdditionalHealth) (Variables|Default|GetAdditionalAttack) (Variables|Default|GetAdditionalSpeed))
    (Actor|DestroyActor)))

(fn ConstructionScript
  (if (!= (Variables|Default|GetAdditionalHealth) 0.0)
    (Rendering|Components|TextRender|SetText (Variables|Default|GetHPStatText) (Utilities|Text|ToText(String) (Utilities|String|Append "HP: " (Utilities|String|ToString(Float) (Variables|Default|GetAdditionalHealth)))))
    (else
      (Rendering|Components|TextRender|SetText (Variables|Default|GetHPStatText) (Utilities|Text|ToText(String) ""))))
  (if (!= (Variables|Default|GetAdditionalAttack) 0.0)
    (Rendering|Components|TextRender|SetText (Variables|Default|GetATKStatText) (Utilities|Text|ToText(String) (Utilities|String|Append "ATK: " (Utilities|String|ToString(Float) (Variables|Default|GetAdditionalAttack)))))
    (else
      (Rendering|Components|TextRender|SetText (Variables|Default|GetATKStatText) (Utilities|Text|ToText(String) ""))))
  (if (!= (Variables|Default|GetAdditionalSpeed) 0.0)
    (Rendering|Components|TextRender|SetText (Variables|Default|GetSPDStatText) (Utilities|Text|ToText(String) (Utilities|String|Append "SPD: " (Utilities|String|ToString(Float) (Variables|Default|GetAdditionalSpeed)))))
    (else
      (Rendering|Components|TextRender|SetText (Variables|Default|GetSPDStatText) (Utilities|Text|ToText(String) "")))))